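; Player controller for multiplayer boat gameplay that spawns and possesses the player's boat, either at a given transform or at a random position.
; On BeginPlay it copies username and flag from the game instance into the game state's arrays and, for local controllers, creates the ranking and dashboard widgets.
; MakeRankingWidget passes name and flag lists to the ranking UI, and Tab prints player-state names for debugging.
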(event Custom|SendPlayerInfos
  (params (pseudo :type String) (flag :type Slate%20Brush%20Structure))
  (bind _output_get (Variables|Default|Setpseudo pseudo))
  (bind _output_get_2 (Variables|Default|Setflag flag))
  (bind _asgs_gameplay_multiplayer (Utilities|Casting|CastToGS_gameplay_multiplayer (Game|GetGameState)))
  (Utilities|Array|Add (Variables|/Game/Multiplayer/GamePlay/GS_gameplay_multiplayer.GS_gameplay_multiplayer_C|Getpseudos _asgs_gameplay_multiplayer) _output_get)
  (Utilities|Array|Add (Variables|/Game/Multiplayer/GamePlay/GS_gameplay_multiplayer.GS_gameplay_multiplayer_C|Getflags _asgs_gameplay_multiplayer) _output_get_2))

(event Custom|GetPlayerInfos
  (bind _asgi_first_version (Utilities|Casting|CastToGI_FirstVersion (Game|GetGameInstance)))
  (CallFunction|SendPlayerInfos (Variables|/Game/NormalGame/GI_FirstVersion.GI_FirstVersion_C|GetUsername _asgi_first_version) (Variables|/Game/NormalGame/GI_FirstVersion.GI_FirstVersion_C|GetNationalityFlag _asgi_first_version)))

(event Custom|MakeRankingWidget
  (params (Pseudos :type Array%20of%20Strings) (Flags :type Array%20of%20Slate%20Brush%20Structures))
  (Default|MakeRanking (Variables|Default|GetUI_ranking) Pseudos Flags))

(event Custom|SpawnOwnBoat
  (params (location :type Transform))
  (if (Pawn|IsLocalController)
    _
    (else
      _))
  (bind _returnvalue (Game|SpawnActorfromClass (Variables|Default|Getclement_pawn) location "AlwaysSpawn" "OverrideRootScale" 0 0.0 0))
  (Pawn|Possess _returnvalue))

(event EventBeginPlay
  (bind _self self)
  (if (Pawn|IsLocalController _self)
    _
    (else
      _))
  (Development|PrintString (Utilities|GetDisplayName _self) true true "(R=1.000000,G=0.920181,B=0.000000,A=1.000000)" 2e+01)
  (CallFunction|GetPlayerInfos)
  (if (Pawn|IsLocalController)
    (bind _returnvalue (UserInterface|CreateWidget "/Game/Multiplayer/GamePlay/UI/UI_ranking.UI_ranking_C" self))
    (bind _output_get (Variables|Default|SetUI_ranking _returnvalue))
    (UserInterface|Viewport|AddtoViewport _output_get 0)
    (bind _returnvalue_2 (UserInterface|CreateWidget "/Game/Multiplayer/GamePlay/UI/TableauDeBord_multi.TableauDeBord_multi_C"))
    (UserInterface|Viewport|AddtoViewport _returnvalue_2 0)))

(event EventTick
  (params (DeltaSeconds :type Float%20%28single-precision%29)))

(event Input|KeyboardEvents|Tab
  (params (Key :type Key%20Structure))
  (bind _returnvalue (Game|GetGameState))
  (bind _playerarray (Variables|/Script/Engine.GameStateBase|GetPlayerArray _returnvalue))
  (:Pressed
    (Development|PrintString "Tab pressed")
    (Development|PrintString (Utilities|String|ToString(Integer) (Utilities|Array|Length _playerarray)))
    (for _array_element _playerarray
      (bind _asps_gameplay_multiplayer (Utilities|Casting|CastToPS_gameplay_multiplayer _array_element))
      (Development|PrintString (Variables|/Game/Multiplayer/GamePlay/PS_gameplay_multiplayer.PS_gameplay_multiplayer_C|Getpseudo _asps_gameplay_multiplayer)))))

(fn ConstructionScript)

(fn SpawnRandomly
  (if (Pawn|IsLocalPlayerController)
    (bind _returnvalue (Game|SpawnActorfromClass (Variables|Default|Getpawn_multi_new_buoyancy) (Math|Transform|MakeTransform (Math|Vector|MakeVector 2e+03 (Math|Random|RandomFloatinRange 0.0 6e+04) 4.6e+03)) "AlwaysSpawn" "OverrideRootScale" self 0.0 0))
    (Pawn|Possess _returnvalue)))