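; Multiplayer game mode for a buoy-course race with wind, which spawns a WindManager and flags the race started after a ten-second timer.
; Joining controllers are queued, and Tick handles one per frame, spawning and possessing a buoyancy pawn at successive GameState spawn points.
; Tick also updates the GameState's controller list and rankings.
; Map retrieval, buoy sorting and start/finish line functions are mostly disconnected or unfinished.
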(event Custom|StartRace
  (Variables|Default|SetRace%20Started true))

(event EventBeginPlay
  (bind _asgs_gameplay_multiplayer (Utilities|Casting|CastToGS_gameplay_multiplayer (Game|GetGameState)))
  (Variables|Default|SetGS _asgs_gameplay_multiplayer)
  (Game|SpawnActorfromClass "/Game/NormalGame/WindManager.WindManager_C" (Math|Transform|MakeTransform "0, 0, 0") "Undefined" "MultiplyWithRoot" 0 0)
  (Utilities|Time|SetTimerbyEvent (delegate Custom|StartRace) 1e+01))

(event EventTick
  (params (DeltaSeconds :type Float%20%28single-precision%29))
  (bind _queue (Variables|Default|Getqueue))
  (bind _output (Utilities|Array|Get(acopy) _queue))
  (if (> (Utilities|Array|Length (Variables|Default|Getqueue)) 0)
    (CallFunction|SpawnPlayer _output)
    (Development|PrintString (Variables|/Game/Multiplayer/GamePlay/PC_gameplay_multiplayer.PC_gameplay_multiplayer_C|Getpseudo _output) true true "(R=1.000000,G=0.000000,B=0.317093,A=1.000000)" 1e+01)
    (Utilities|Array|RemoveItem (Variables|Default|Getqueue) _output)
    (Utilities|Array|Add (Variables|/Game/Multiplayer/GamePlay/GS_gameplay_multiplayer.GS_gameplay_multiplayer_C|Getcontrollers (Variables|Default|GetGS)) _output)
    (Default|MakeRankings (Variables|Default|GetGS))))

(event EventHandleStartingNewPlayer
  (params (NewPlayer :type Player%20Controller%20Object%20Reference))
  (bind _aspc_gameplay_multiplayer (Utilities|Casting|CastToPC_gameplay_multiplayer NewPlayer))
  (Utilities|Array|Add (Variables|Default|Getqueue) _aspc_gameplay_multiplayer)
  (Development|PrintString "NEW STARTING PLAYER" true true "(R=1.000000,G=0.520103,B=0.000000,A=1.000000)" 2e+01))

(fn ConstructionScript)

(fn RetrieveMap
  (params (SG :type Save%20Game%20Object%20Reference))
  (bind _assg_map_editor (Utilities|Casting|CastToSG_MapEditor SG)))

(fn MakeStartLine
  (bind _outactors (Actor|GetAllActorsOfClass 0)))

(fn DrawStartLine)

(fn MakeFinishLine
  (bind _outactors (Actor|GetAllActorsOfClass 0)))

(fn DrawFinishLine
  (Rendering|Debug|DrawDebugLine (+ (Transformation|GetActorLocation) "0.000000,0.000000,300.000000") (+ (Transformation|GetActorLocation) "0.000000,0.000000,300.000000") (Class|KismetMathLibrary|LinearColorRed) 1e+02 1.5e+02))

(fn SortBuoys
  (Actor|GetAllActorsOfClass 0))

(fn GetPositiononWater
  (params (NewParam :type Vector))
  (bind _outhit (Collision|LineTraceForObjects (+ NewParam "0.000000,0.000000,5000.000000") (+ NewParam "0.000000,0.000000,-5000.000000") (Utilities|Array|MakeArray "ObjectTypeQuery1") false 0 "None"))
  (return (Math|Conversions|ToTransform(Vector) (+ (.ImpactPoint (Collision|BreakHitResult _outhit)) "0.000000,0.000000,450.000000"))))

(fn SpawnPlayer
  (params (PlayerController :type PC%20Gameplay%20Multiplayer%20Object%20Reference))
  (Development|PrintString "SpawnPlayerCalled" true true "(R=1.000000,G=0.093488,B=0.000000,A=1.000000)" 1e+01)
  (LocalVariables|SetLocalController PlayerController)
  (bind _returnvalue (Game|SpawnActorfromClass (Variables|Default|Getpawn_multi_new_buoyancy) (Math|Transform|MakeTransform (+ (Utilities|Array|Get(acopy) (Variables|/Game/Multiplayer/GamePlay/GS_gameplay_multiplayer.GS_gameplay_multiplayer_C|GetSpawn%20Points (Variables|Default|GetGS)) (Variables|Default|GetSpawnNumber)) "0.000000,0.000000,-400.000000") "0.000000,90.000000,0.000000") "AlwaysSpawn" "OverrideRootScale" 0 0.0 0))
  (Pawn|Possess (LocalVariables|GetLocalController) _returnvalue)
  (Variables|Default|SetSpawnNumber (+ (Variables|Default|GetSpawnNumber) 1)))

(fn AddPlayeronData
  (params (Controller :type PC%20Gameplay%20Multiplayer%20Object%20Reference))
  (bind _gs (Variables|Default|GetGS))
  (Default|GetPlayerInfos Controller)
  (Utilities|Array|Add (Variables|/Game/Multiplayer/GamePlay/GS_gameplay_multiplayer.GS_gameplay_multiplayer_C|Getpseudos _gs) "")
  (Utilities|Array|Add :TargetArray (Variables|/Game/Multiplayer/GamePlay/GS_gameplay_multiplayer.GS_gameplay_multiplayer_C|Getflags _gs))
  (Utilities|Array|Add (Variables|/Game/Multiplayer/GamePlay/GS_gameplay_multiplayer.GS_gameplay_multiplayer_C|Getcontrollers _gs) Controller)
  (Default|MakeRankings (Variables|Default|GetGS)))