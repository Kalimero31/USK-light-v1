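; Game mode for solo play that, as wired, only caches spawn points at BeginPlay from the first GS_solo actor found in the world.
; HandleStartingNewPlayer is overridden but empty, so it does no player setup.
; Disconnected logic would collect player controllers and, at exactly three players, spawn and possess a PAWN_AC68 boat for each at its indexed spawn point.
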(event EventBeginPlay
  (bind _outactors (Actor|GetAllActorsOfClass "/Game/NormalGame/GS_solo.GS_solo_C"))
  (bind _output_get (Variables|Default|SetSpawnPoints (Variables|/Game/NormalGame/GS_solo.GS_solo_C|GetSpawnPoints (Utilities|Array|Get(acopy) _outactors)))))

(event EventTick
  (params (DeltaSeconds :type Float%20%28single-precision%29)))

(event EventHandleStartingNewPlayer
  (params (NewPlayer :type Player%20Controller%20Object%20Reference)))

(fn ConstructionScript)