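; Umpire-testing player controller that lets the player switch between two animated AC68 boat pawns.
; On BeginPlay it gathers all PAWN_AC68_animated actors in the level and possesses the first one found.
; Space Bar uses the CurrentBoatA flag to alternate possession between the first two boats, calling ResetView on the boat it takes over.
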(event EventBeginPlay
  (bind _outactors (Actor|GetAllActorsOfClass "/Game/Boats/AC_68/Pawn/PAWN_AC68_animated.PAWN_AC68_animated_C"))
  (bind _output_get (Variables|Default|Setboats _outactors))
  (Pawn|Possess (Utilities|Array|Get(acopy) _output_get)))

(event EventTick
  (params (DeltaSeconds :type Float%20%28single-precision%29)))

(event Input|KeyboardEvents|SpaceBar
  (params (Key :type Key%20Structure :default "None"))
  (bind _boats (Variables|Default|Getboats))
  (bind _boats_2 (Variables|Default|Getboats))
  (bind _output (Utilities|Array|Get(acopy) _boats_2))
  (bind _output_2 (Utilities|Array|Get(acopy) _boats 1))
  (:Pressed
    (if (Variables|Default|GetCurrentBoatA)
      (Pawn|Possess _output_2)
      (Default|ResetView _output_2)
      (Variables|Default|SetCurrentBoatA false)
      (else
        (Pawn|Possess _output)
        (Default|ResetView _output)
        (Variables|Default|SetCurrentBoatA true)))))

(fn ConstructionScript)